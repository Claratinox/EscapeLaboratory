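; AC_0X00A21E is an actor component in the science lab security system that acts on whichever actor owns it.
; On BeginPlay it sets DetectMode to true, so its branch always passes, and disables collision on an owning BP_LabDoor01.
; Its separate EOT event applies the PP_EndOfTransmission post-process blendable at full weight to an owning BP_Body's first-person camera.
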(event Custom|EOT
  ;[1 0 0] FatalError 0x00CE124
  (bind _asbp_body (Utilities|Casting|CastToBP_Body (Components|GetOwner)))
  (Variables|/Script/Engine.CameraComponent|SetPostProcessSettings (Variables|/Game/EurileneGene/Core/BP_Body.BP_Body_C|GetFirstPersonCamera _asbp_body) (Utilities|Struct|MakePostProcessSettings (Utilities|Struct|MakeWeightedBlendables (Utilities|Array|MakeArray (Utilities|Struct|MakeWeightedBlendable 1.0 "/Game/ScienceLab/SecuritySystem/PP_EndOfTransmission.PP_EndOfTransmission"))))))

(event EventBeginPlay
  ;[0 0.3281 0] Really protected, don't touch plz ! :(
  (Variables|Default|SetDetectMode true)
  (if (Variables|Default|GetDetectMode)
    (bind _asbp_lab_door_01 (Utilities|Casting|CastToBP_LabDoor01 (Components|GetOwner)))
    (Collision|SetCollisionEnabled (Variables|/Game/ScienceLab/Blueprints/Rooms/Doors/BP_LabDoor01.BP_LabDoor01_C|GetCollision _asbp_lab_door_01) "NoCollision")))

(event EventTick
  (params (DeltaSeconds :type Float%20%28single-precision%29)))